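; BP_PickupAmmo is a collectable pickup that refills reserve ammo for the first-person character's weapons.
; On Collect, it loops through every weapon in the character's WeaponArray and adds a fixed amount to AmmoStorage, clamped to that weapon's MaxAmmoStorage.
; Each new storage value is printed on screen as debug output.
; BeginPlay and the construction script only call their parent versions.
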(event `self.ReceiveBeginPlay`
  (`parent.ReceiveBeginPlay`))

(event `self.Collect`
  (for _array_element (`/Game/_Core/Blueprints/BP_FirstPersonCharacter.WeaponArray` (`self.As BP First Person Character`))
    (bind _output_get (set `/Game/_Core/Blueprints/Weapons/BP_WeaponBase.AmmoStorage` (`KismetMathLibrary.Clamp` (+ (`/Game/_Core/Blueprints/Weapons/BP_WeaponBase.AmmoStorage` _array_element) 5) 0 (`/Game/_Core/Blueprints/Weapons/BP_WeaponBase.MaxAmmoStorage` _array_element)) _array_element))
    (`KismetSystemLibrary.PrintString` (`KismetStringLibrary.Conv_IntToString` _output_get))))

(fn `UserConstructionScript`
  (`parent.UserConstructionScript`))