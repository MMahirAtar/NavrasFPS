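; Sniper rifle weapon Blueprint that adds a toggleable 2x scope to its parent weapon class.
; Alternative use flips the scope state between unscoped and 2x, then switches player 0's view target between the pawn and the weapon actor itself.
; A weapon change resets the scope if this weapon is active and is the current view target.
; Firing, reloading and ammo spending defer to the parent.
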(event `self.OnFireProjectile`
  (`parent.OnFireProjectile`))

(event `self.ReloadWeapon`
  (`parent.ReloadWeapon`))

(event `self.SpendAmmo`
  (`parent.SpendAmmo`))

(event `self.UseAlternative`
  (set `self.scopeState` (select `/Game/_Core/Blueprints/EScopeState` (`self.scopeState`) :`NewEnumerator0` "NewEnumerator1" :`NewEnumerator1` "NewEnumerator0" :!type "/Game/_Core/Blueprints/EScopeState Enum"))
  (`self.ToggleScope`))

(event `ToggleScope`
  (bind _returnvalue (`GameplayStatics.GetPlayerController` 0))
  (if (`self.IsActive`)
    (switch `/Game/_Core/Blueprints/EScopeState` (`self.scopeState`)
      (:`NewEnumerator0`
        (`PlayerController.SetViewTargetWithBlend` _returnvalue (`GameplayStatics.GetPlayerPawn` 0) 0.0 "VTBlend_Linear" 0.0 false))
      (:`NewEnumerator1`
        (`PlayerController.SetViewTargetWithBlend` _returnvalue self 0.0 "VTBlend_Linear" 0.0 false)))))

(event `self.OnWeaponChanged`
  (if (`self.IsActive`)
    (if (== (`Controller.GetViewTarget` (`GameplayStatics.GetPlayerController` 0)) self)
      (set `self.scopeState` "NewEnumerator0")
      (`self.ToggleScope`))))

(fn `UserConstructionScript`
  (`parent.UserConstructionScript`))