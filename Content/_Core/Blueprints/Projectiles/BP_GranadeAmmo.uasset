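; Grenade projectile that deals area damage to nearby enemies shortly after its first impact.
; On the first hit it waits a second, runs a physics interaction on the struck component, then sphere-overlaps enemy pawns around the hit location.
; Each enemy with a BPC_Health component takes the grenade's damage and has its name printed before the projectile destroys itself.
; Disconnected leftovers hold an older trace-based damage pass and a character knockback launch.
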(event `self.ReceiveHit`
  (params (MyComp :type "PrimitiveComponent Object Reference") (Other :type "Actor Object Reference") (OtherComp :type "PrimitiveComponent Object Reference") (bSelfMoved :type Boolean) (HitLocation :type "Vector Structure") (HitNormal :type "Vector Structure") (NormalImpulse :type "Vector Structure") (Hit :type "HitResult Structure (by ref)"))
  (`/Engine/EditorBlueprintResources/StandardMacros.DoOnce` false
    (:`Completed`
      (`KismetSystemLibrary.Delay` 1.0)
      (`self.Physics Interaction` OtherComp)
      (bind _outactors (`KismetSystemLibrary.SphereOverlapActors` HitLocation 750.0 (`|MakeArray` "ObjectTypeQuery3" :!type "EObjectTypeQuery Enum") "/Game/_Core/Blueprints/Characters/BP_EnemyBase.BP_EnemyBase_C"))
      (for _array_element _outactors
        (bind _returnvalue (`self.GetComponentByClass` _array_element "/Game/_Core/Blueprints/Components/BPC_Health.BPC_Health_C"))
        (`/Engine/EditorBlueprintResources/StandardMacros.IsValid` _returnvalue
          (:`Is Valid`
            (`/Game/_Core/Blueprints/Components/BPC_Health.GainDamage` _returnvalue (`self.Damage`))
            (`KismetSystemLibrary.PrintString` (`KismetSystemLibrary.GetDisplayName` _array_element)))))
      (`self.K2_DestroyActor`))))

(fn `UserConstructionScript`
  (`parent.UserConstructionScript`))