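; Health component that tracks an actor's current health and alive state, starting at full health on BeginPlay.
; GainHealth and GainDamage act only while alive, clamp health between zero and MaxHealth, and call OnGainHealth or OnDamage.
; When damage brings health to zero, a DoOnce gate calls OnDied and clears IsAlive, blocking further changes.
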(event `self.ReceiveBeginPlay`
  (set `self.CurrentHealth` (`self.MaxHealth`))
  (set `self.IsAlive` true))

(event `GainHealth`
  (params (CurrentHealth :type Integer))
  (if (`self.IsAlive`)
    (set `self.CurrentHealth` (`KismetMathLibrary.Clamp` (+ CurrentHealth (`self.CurrentHealth`)) 0 (`self.MaxHealth`)))
    (`self.OnGainHealth`)))

(event `GainDamage`
  (params (`Damage Amount` :type Integer))
  (if (`self.IsAlive`)
    (set `self.CurrentHealth` (`KismetMathLibrary.Clamp` (- (`self.CurrentHealth`) `Damage Amount`) 0 (`self.MaxHealth`)))
    (`self.OnDamage`)
    (if (== (`self.CurrentHealth`) 0)
      (`/Engine/EditorBlueprintResources/StandardMacros.DoOnce` false
        (:`Completed`
          (`self.On Died`)
          (set `self.IsAlive` false))))))