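; BP_MeleAttacker is a melee enemy character that chases the player and punches, then goes ragdoll on death.
; Its looping timer and Root event suggest a polled Idle/Chase/Attack state machine, with pawn sensing or taking damage triggering chases.
; Reaching the destination triggers a left-hook montage and returns to idle.
; While IsAttacking, Tick sphere-traces the left forearm, damaging the player's BPC_Health once until ResetAttack.
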(event `self.ReceiveBeginPlay`
  (`parent.ReceiveBeginPlay`)
  (`KismetSystemLibrary.K2_SetTimerDelegate` (`|CreateDelegate` :!event `Root`) 0.03 (`self.IsAlive`))
  (set `self.Start pos ` (`self.K2_GetActorLocation`)))

(event `Root`
  (if (`self.IsAlive`)
    (switch `/Game/_Core/Blueprints/AI/EEnemyState` (`self.State`)
      (:`NewEnumerator0`
        (`MovementComponent.StopMovementImmediately` (`self.CharacterMovement`)))
      (:`NewEnumerator1`
        (`self.Attack `))
      (:`NewEnumerator2`
        (`|AIMoveTo` self (`self.Destination`) null 50.0 true
          (:`OnSuccess`
            (set `self.State` "NewEnumerator1")))))))

(event `self.PawnSensing.OnSeePawn`
  (params (Pawn :type "Pawn Object Reference"))
  (if (`self.IsAlive`)
    (if (not (`|EnumEquality` (`self.State`) "NewEnumerator1"))
      (bind _asbp_first_person_character (cast `/Game/_Core/Blueprints/BP_FirstPersonCharacter` Pawn))
      (set `self.Player` _asbp_first_person_character)
      (set `self.State` "NewEnumerator2")
      (set `self.Destination` (`self.K2_GetActorLocation` (`self.Player`))))))

(event `Attack`
  (`self.PlayAnimMontage` "/Game/Characters/Mannequins/Animations/Attack/NinjaLeftHook_Montage.NinjaLeftHook_Montage")
  (set `self.State` "NewEnumerator0"))

(event `self.OnDied`
  (set `self.IsAlive` false)
  (`PrimitiveComponent.SetCollisionEnabled` (`self.CapsuleComponent`) "NoCollision")
  (`ActorComponent.Deactivate` (`self.PawnSensing`))
  (set `self.State` "NewEnumerator0")
  (`PrimitiveComponent.SetSimulatePhysics` (`self.Mesh`) true)
  (`SkeletalMeshComponent.SetAllBodiesPhysicsBlendWeight` (`self.Mesh`) 1.0 false))

(event `self.OnGainDamage`
  (set `self.Destination` (`self.K2_GetActorLocation` (`GameplayStatics.GetPlayerPawn` 0)))
  (set `self.State` "NewEnumerator2"))

(event `self.ReceiveTick`
  (params (DeltaSeconds :type "Float (single-precision)"))
  (bind _mesh (`self.Mesh`))
  (bind _returnvalue (`self.GetComponentByClass` (`self.Hit Actor`) "/Game/_Core/Blueprints/Components/BPC_Health.BPC_Health_C"))
  (if (`self.IsAttacking`)
    (bind _outhits (`KismetSystemLibrary.SphereTraceMultiForObjects` :`Start` (`SceneComponent.GetSocketLocation` _mesh "hand_l") :`End` (`SceneComponent.GetSocketLocation` _mesh "lowerarm_l") :`Radius` 20.0 :`ObjectTypes` (`|MakeArray` "ObjectTypeQuery3" :!type "EObjectTypeQuery Enum") :`DrawDebugType` "ForOneFrame"))
    (for _array_element _outhits
      (bind (_bblockinghit _binitialoverlap _time _distance _location _impactpoint _normal _impactnormal _physmat _hitactor) (`GameplayStatics.BreakHitResult` _array_element))
      (if _bblockinghit
        (set `self.Hit Actor` _hitactor)
        (if (`self.ActorHasTag` (`self.Hit Actor`) "Player")
          (`/Engine/EditorBlueprintResources/StandardMacros.DoOnce` false :!label _label
            (:`Completed`
              (`/Engine/EditorBlueprintResources/StandardMacros.IsValid` _returnvalue
                (:`Is Valid`
                  (`/Game/_Core/Blueprints/Components/BPC_Health.GainDamage` _returnvalue (`self.Damage Amount`))
                  (`KismetSystemLibrary.PrintString` (`KismetStringLibrary.Conv_IntToString` (`/Game/_Core/Blueprints/Components/BPC_Health.CurrentHealth` _returnvalue))))))))))))

(event `ResetAttack`
  (goto _label :!via `Reset`))

(fn `UserConstructionScript`
  (`parent.UserConstructionScript`))