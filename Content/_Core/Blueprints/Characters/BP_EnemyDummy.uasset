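; BP_EnemyDummy is an enemy dummy character that displays its current health as text.
; Every tick it copies CurrentHealth from its BPCHealth component into a TextRender as an integer.
; OnDied hides only the mesh, without propagating to child components or destroying the actor.
; The PawnSensing OnSeePawn event is present but empty, so the dummy has no reaction to seen pawns.
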(event `self.ReceiveTick`
  (params (DeltaSeconds :type "Float (single-precision)"))
  (`TextRenderComponent.K2_SetText` (`self.TextRender`) (`KismetTextLibrary.Conv_IntToText` (`/Game/_Core/Blueprints/Components/BPC_Health.CurrentHealth` (`self.BPC_Health`)))))

(event `self.OnDied`
  (`SceneComponent.SetVisibility` (`self.Mesh`) false false))

(event `self.PawnSensing.OnSeePawn`
  (params (Pawn :type "Pawn Object Reference")))

(fn `UserConstructionScript`
  (`parent.UserConstructionScript`))